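; Player Blueprint that applies a direction-specific physical reaction to the target enemy on each attack event.
; OnAttack caches the enemy and a flattened direction to it, then switches on attack type.
; Timelines drive the squash, carry and spins, while impulse-like AddForce calls pull, push or launch the enemy's capsule.
; The Left attack suspends physics while moving the enemy, then chains into the Above squash; completed branches call FinishAttack.
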(event `self.ReceiveBeginPlay`
  (add `self.OnAttack` (delegate `OnAttackEvent`)))

(event `OnAttackEvent` :!signature `self.OnAttack`
  (params (Enemy :type "Enemy Object Reference") (AttackType :type "EAttackType Enum" :default "Above"))
  (bind (_returnvalue_roll _returnvalue_pitch _returnvalue_yaw) (`KismetMathLibrary.BreakRotator` (`self.K2_GetActorRotation` (`self.CurrentEnemy`))))
  (bind (_returnvalue_roll_2 _returnvalue_pitch_2 _returnvalue_yaw_2) (`KismetMathLibrary.BreakRotator` (`self.K2_GetActorRotation` (`self.CurrentEnemy`))))
  (bind (_returnvalue_x _returnvalue_y) (`KismetMathLibrary.BreakVector` (- (`self.K2_GetActorLocation` Enemy) (`self.K2_GetActorLocation`))))
  (`/Engine/EditorBlueprintResources/StandardMacros.IsValid` Enemy
    (:`Is Valid`
      (set `self.CurrentEnemy` Enemy)
      (set `self.DirToEnemy` (`KismetMathLibrary.Normal` (`KismetMathLibrary.MakeVector` _returnvalue_x _returnvalue_y)))
      (switch `EAttackType` AttackType
        (:`Above`
          ;[1 1 1] Above attack
          (`SceneComponent.SetWorldScale3D` (`Character.CapsuleComponent` (`self.CurrentEnemy`)) (1.0 1.0 0.5) :!label _label)
          (`Timeline|AboveAttackTimeline` :!via `PlayFromStart`
            (:`Finished`
              (`/Engine/EditorBlueprintResources/StandardMacros.IsValid` (`self.CurrentEnemy`)
                (:`Is Valid`
                  (`SceneComponent.SetWorldScale3D` (`Character.CapsuleComponent` (`self.CurrentEnemy`)) (1.0 1.0 1.0)))
                (:`Is Not Valid`
                  _))
              (`self.FinishAttack`))))
        (:`Below`
          ;[1 1 1] Below attack
          (`PrimitiveComponent.AddForce` (`Character.CapsuleComponent` (`self.CurrentEnemy`)) (* (`KismetMathLibrary.NegateVector` (`self.DirToEnemy`)) (`self.BelowAttackPower`)) "None" false)
          (`self.FinishAttack`))
        (:`Left`
          ;[1 1 1] Left attack
          (`PrimitiveComponent.SetSimulatePhysics` (`Character.CapsuleComponent` (`self.CurrentEnemy`)) false)
          (bind (_direction _yloc _zloc) (`Timeline|LeftAttackTimeline` :!via `PlayFromStart`)
            (:`Update`
              (`/Engine/EditorBlueprintResources/StandardMacros.IsValid` (`self.CurrentEnemy`)
                (:`Is Valid`
                  (`self.K2_SetActorLocation` (`self.CurrentEnemy`) (+ (+ (`self.K2_GetActorLocation`) (`KismetMathLibrary.MakeVector` 0.0 0.0 _zloc)) (* (`self.DirToEnemy`) _yloc)) true false))))
            (:`Finished`
              (`/Engine/EditorBlueprintResources/StandardMacros.IsValid` (`self.CurrentEnemy`)
                (:`Is Valid`
                  (`PrimitiveComponent.SetSimulatePhysics` (`Character.CapsuleComponent` (`self.CurrentEnemy`)) true)
                  (goto _label))
                (:`Is Not Valid`
                  (`self.FinishAttack`))))))
        (:`Right`
          ;[1 1 1] Right attack
          (set `self.CurrentEnemyStartZRot` _returnvalue_yaw)
          (bind (_direction_2 _zrotdelta) (`Timeline|RightAttackTimeline` :!via `PlayFromStart`)
            (:`Update`
              (`/Engine/EditorBlueprintResources/StandardMacros.IsValid` (`self.CurrentEnemy`)
                (:`Is Valid`
                  (`self.K2_SetActorRotation` (`self.CurrentEnemy`) (`KismetMathLibrary.MakeRotator` 0.0 0.0 (+ (`self.CurrentEnemyStartZRot`) _zrotdelta)) false))))
            (:`Finished`
              (`self.FinishAttack`))))
        (:`Ahead`
          ;[1 1 1] Ahead attack
          (`PrimitiveComponent.AddForce` (`Character.CapsuleComponent` (`self.CurrentEnemy`)) (* (`self.DirToEnemy`) (`self.AheadAttackPower`)) "None" false)
          (bind (_direction_3 _rotspeed) (`Timeline|AheadAttackTimeline` :!via `PlayFromStart`)
            (:`Update`
              (`/Engine/EditorBlueprintResources/StandardMacros.IsValid` (`self.CurrentEnemy`)
                (:`Is Valid`
                  (`self.K2_SetActorRotation` (`self.CurrentEnemy`) (`KismetMathLibrary.MakeRotator` 0.0 0.0 (+ _returnvalue_yaw_2 (* _rotspeed 10.0))) false))))
            (:`Finished`
              (`self.FinishAttack`))))
        (:`Behind`
          ;[1 1 1] Behind attack
          (`PrimitiveComponent.AddForce` (`Character.CapsuleComponent` (`self.CurrentEnemy`)) (* (`KismetMathLibrary.RotateAngleAxis` (`self.DirToEnemy`) 45.0 (0.0 1.0 0.0)) (`self.BehindAttackPower`)) "None" false)
          (`self.FinishAttack`))))
    (:`Is Not Valid`
      (`self.FinishAttack`))))

(fn `UserConstructionScript`)